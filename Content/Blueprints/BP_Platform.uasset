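; BP_Platform is a pooled platform actor that appears for a fixed, short lifetime and then recycles itself.
; On initialisation it stores a reference to its object pool.
; On activation it enables visibility, tick and mesh collision, waits on a Delay, then disables all three and returns itself to the pool.
; The deactivation event is empty, since that teardown runs inline after the delay.
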(event EventBeginPlay)

(event Collision|EventActorBeginOverlap
  (params (OtherActor :type Actor%20Object%20Reference)))

(event EventTick
  (params (DeltaSeconds :type Float%20%28single-precision%29)))

(event EventOnInitialisation
  (params (ObjectPoolRef :type BP%20Object%20Pool%20Object%20Reference))
  (Variables|Default|SetObject%20Pool%20Ref ObjectPoolRef))

(event EventOnDeactivation)

(event EventOnActivation
  (Rendering|SetActorHiddenInGame false)
  (Actor|Tick|SetActorTickEnabled true)
  (Collision|SetCollisionEnabled (Variables|Default|GetStaticMesh) "QueryAndPhysics")
  (Utilities|FlowControl|Delay 5.0)
  (Rendering|SetActorHiddenInGame true)
  (Actor|Tick|SetActorTickEnabled false)
  (Collision|SetCollisionEnabled (Variables|Default|GetStaticMesh) "NoCollision")
  (Default|ReturntoPool (Variables|Default|GetObject%20Pool%20Ref) self))

(fn ConstructionScript)