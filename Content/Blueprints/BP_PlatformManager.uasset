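; BP_PlatformManager extends a line of platforms by periodically placing pooled actors along the world X axis.
; On BeginPlay it finds the BP_ObjectPool and takes an existing BP_Platform's transform as the starting point, then starts a looping timer, cleared on EndPlay.
; SpawnPlatform takes an actor from the pool, teleports it a fixed step beyond the last position, prints the transform and sends it an activation message.
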(event Custom|SpawnPlatform
  (bind _returnactor (Default|TakefromPool (Variables|Default|GetObjectPool)))
  (Utilities|IsValid _returnactor
    (:Is%20Valid
      (bind _output_get (Variables|Default|SetSpawnTransform (Math|Transform|MakeTransform (Math|Vector|MakeVector (+ (.X (Math|Vector|BreakVector (.Location (Math|Transform|BreakTransform (Variables|Default|GetSpawnTransform))))) 1e+03) (.Y (Math|Vector|BreakVector (.Location (Math|Transform|BreakTransform (Variables|Default|GetSpawnTransform))))) (.Z (Math|Vector|BreakVector (.Location (Math|Transform|BreakTransform (Variables|Default|GetSpawnTransform)))))) (.Rotation (Math|Transform|BreakTransform (Variables|Default|GetSpawnTransform))) (.Scale (Math|Transform|BreakTransform (Variables|Default|GetSpawnTransform))))))
      (Transformation|Teleport _returnactor (.Location (Math|Transform|BreakTransform _output_get)) (.Rotation (Math|Transform|BreakTransform _output_get)))
      (Development|PrintString (Utilities|String|ToString(Transform) _output_get))
      (Class|BPIPoolObject|OnActivation(Message) _returnactor))))

(event EventBeginPlay
  (bind _outactors (Actor|GetAllActorsOfClass "/Game/Blueprints/BP_ObjectPool.BP_ObjectPool_C"))
  (Utilities|IsValid (Utilities|Array|Get(acopy) _outactors)
    (:Is%20Valid
      (Variables|Default|SetObjectPool (Utilities|Array|Get(acopy) _outactors))
      (bind _outactors_2 (Actor|GetAllActorsOfClass "/Game/Blueprints/BP_Platform.BP_Platform_C"))
      (Utilities|IsValid (Utilities|Array|Get(acopy) _outactors_2)
        (:Is%20Valid
          (Variables|Default|SetSpawnTransform (Transformation|GetActorTransform (Utilities|Array|Get(acopy) _outactors_2)))
          (bind _returnvalue (Utilities|Time|SetTimerbyEvent (EventDispatchers|CreateEvent :!event Custom|SpawnPlatform) 4.0 true))
          (Variables|Default|SetspawnTimerHandle _returnvalue))))))

(event EventEndPlay
  (params (EndPlayReason :type EEndPlayReason%20Enum :default "Destroyed"))
  (Utilities|Time|ClearandInvalidateTimerbyHandle (Variables|Default|GetspawnTimerHandle)))

(fn ConstructionScript)