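; BP_ObjectPool is an actor pool that pre-spawns SpawnClass actors on BeginPlay, hides them, disables their tick and messages each with a pool reference.
; TakeFromPool removes index 0, then reads index 0 for return, without re-enabling the actor.
; Its WillGrow spawn follows that return inside the non-empty branch, so an empty pool never grows.
; ReturnToPool re-adds valid actors without hiding them; both functions print pool size.
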(event EventBeginPlay
  (for _index (range 0 (- (Variables|Default|GetPoolSize) 0))
    (bind _returnvalue (Game|SpawnActorfromClass (Variables|Default|GetSpawnClass) (Math|Transform|MakeTransform "0, 0, 0") "AlwaysSpawn" "MultiplyWithRoot" 0 0))
    (CallFunction|AddtoPool _returnvalue)
    (Class|BPIPoolObject|OnInitialisation(Message) _returnvalue self)))

(event Collision|EventActorBeginOverlap
  (params (OtherActor :type Actor%20Object%20Reference)))

(event EventTick
  (params (DeltaSeconds :type Float%20%28single-precision%29)))

(fn ConstructionScript)

(fn AddtoPool
  (params (ActorToAdd :type Actor%20Object%20Reference))
  (Utilities|Array|Add (Variables|Default|GetPoolActors) ActorToAdd)
  (Rendering|SetActorHiddenInGame ActorToAdd true)
  (Actor|Tick|SetActorTickEnabled ActorToAdd))

(fn TakefromPool
  (if (> (Utilities|Array|Length (Variables|Default|GetPoolActors)) 0)
    (Utilities|FlowControl|Sequence
      (:then_0
        (Utilities|Array|RemoveIndex (Variables|Default|GetPoolActors))
        (Development|PrintString (Utilities|String|Append "The Array Length is: " (Utilities|String|ToString(Integer) (Utilities|Array|Length (Variables|Default|GetPoolActors)))))
        (return (Utilities|Array|Get(acopy) (Variables|Default|GetPoolActors))))
      (:then_1
        (if (Variables|Default|GetWillGrow)
          (bind _returnvalue (Game|SpawnActorfromClass (Variables|Default|GetSpawnClass) (Math|Transform|MakeTransform "0, 0, 0") "Undefined" "MultiplyWithRoot" 0 0))
          (return _returnvalue)
          (else
            (return 0)))))
    (else
      (return 0))))

(fn ReturntoPool
  (params (ActorToReturn :type Actor%20Object%20Reference))
  (Utilities|IsValid ActorToReturn
    (:Is%20Valid
      (Utilities|Array|Add (Variables|Default|GetPoolActors) ActorToReturn)
      (Development|PrintString (Utilities|String|Append "The Array Length after returning an object is: " (Utilities|String|ToString(Integer) (Utilities|Array|Length (Variables|Default|GetPoolActors))))))))